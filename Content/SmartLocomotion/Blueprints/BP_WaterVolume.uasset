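; BP_WaterVolume is a water volume actor that puts overlapping Characters into swimming.
; On begin overlap of its collision box, it flags the movement component's current physics volume as water and sets the movement mode to Swimming.
; End overlap only clears that water flag, without setting a new mode.
; A helper function, uncalled here, line-traces below a character with persistent debug drawing.
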(event OnComponentBeginOverlap(ColisionBox)
  (params (OverlappedComponent :type Primitive%20Component%20Object%20Reference) (OtherActor :type Actor%20Object%20Reference) (OtherComp :type Primitive%20Component%20Object%20Reference) (OtherBodyIndex :type Integer) (bFromSweep :type Boolean) (SweepResult :type Hit%20Result%20Structure%20%28by%20ref%29))
  ;[0 0 0] Begin Overlap
  (bind _ascharacter (Utilities|Casting|CastToCharacter OtherActor))
  (Variables|/Script/Engine.PhysicsVolume|SetbWaterVolume (Class|MovementComponent|GetPhysicsVolume (Variables|/Script/Engine.Character|GetCharacterMovement _ascharacter)) true)
  (Pawn|Components|CharacterMovement|SetMovementMode (Variables|/Script/Engine.Character|GetCharacterMovement _ascharacter) "MOVE_Swimming" 0))

(event OnComponentEndOverlap(ColisionBox)
  (params (OverlappedComponent :type Primitive%20Component%20Object%20Reference) (OtherActor :type Actor%20Object%20Reference) (OtherComp :type Primitive%20Component%20Object%20Reference) (OtherBodyIndex :type Integer))
  ;[0 0 0] End Overlap
  (bind _ascharacter (Utilities|Casting|CastToCharacter OtherActor))
  (Variables|/Script/Engine.PhysicsVolume|SetbWaterVolume (Class|MovementComponent|GetPhysicsVolume (Variables|/Script/Engine.Character|GetCharacterMovement _ascharacter)) false))

(fn ConstructionScript)

(fn TraceUnderFeet
  (params (Character :type Character%20Object%20Reference))
  (bind _returnvalue (Transformation|GetActorLocation Character))
  (bind _returnvalue_2 (Collision|LineTraceByChannel _returnvalue (- _returnvalue "0, 0,100.000000") "TraceTypeQuery1" false 0 "Persistent"))
  (return _returnvalue_2))