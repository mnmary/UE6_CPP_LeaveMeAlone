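; Player controller for LeaveMeAlone that opens the pause menu and the end-of-game screen.
; The Pause input, guarded by an OnPause flag, pauses the game and shows WBP_Pause with UI-only input and a visible cursor.
; UnPossess, treated as character death, starts a short timer whose DeathEvent pauses the game and shows WBP_EndOfGame the same way.
; Nothing in this controller resumes play or clears OnPause.
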(event Custom|DeathEvent
  ;[1 1 1] Вызов меню, после смерти персонажа c помощью таймера
  (Utilities|Time|ClearandInvalidateTimerbyHandle (Variables|Default|GetDeadTimer))
  (Game|SetGamePaused true)
  (bind _returnvalue (UserInterface|CreateWidget "/Game/LeaveMeAlone/Widgets/UI/WBP_EndOfGame.WBP_EndOfGame_C"))
  (UserInterface|Viewport|AddtoViewport _returnvalue 0)
  (Input|SetInputModeUIOnly self _returnvalue "DoNotLock" false)
  (Variables|Default|SetbShowMouseCursor true))

(event EventBeginPlay)

(event EventTick
  (params (DeltaSeconds :type Float%20%28single-precision%29)))

(event EventUnPossess
  (params (UnpossessedPawn :type Pawn%20Object%20Reference))
  ;[1 1 1] Вызов меню, после смерти персонажа c помощью таймера
  (bind _returnvalue (Utilities|Time|SetTimerbyEvent (delegate Custom|DeathEvent) 3.0))
  (Variables|Default|SetDeadTimer _returnvalue))

(event Input|ActionEvents|InputActionPause
  (params (Key :type Key%20Structure :default "None"))
  ;[0.15 0.15 0.15 0.5] Обрабатывавем нажатие паузы
  (:Pressed
    (if (not (Variables|Default|GetOnPause))
      (bind _output_get (Variables|Default|SetOnPause true))
      (Game|SetGamePaused true)
      (bind _returnvalue (UserInterface|CreateWidget "/Game/LeaveMeAlone/Widgets/UI/WBP_Pause.WBP_Pause_C"))
      (bind _output_get_2 (Variables|Default|SetPauseWidget _returnvalue))
      (UserInterface|Viewport|AddtoViewport _output_get_2 0)
      (Input|SetInputModeUIOnly self _output_get_2 "DoNotLock" false)
      (Variables|Default|SetbShowMouseCursor true)
      (Development|PrintString "set pause" _output_get))))

(fn ConstructionScript)