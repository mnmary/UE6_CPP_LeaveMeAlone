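; Game mode for LeaveMeAlone that runs the match countdown and shows the end-of-game screen.
; A looping one-second timer started on BeginPlay decrements GameTime.
; At zero it clears the timer, adds WBP_EndOfGame to the viewport and switches the player controller to game-and-UI input focused on that widget.
; An unconnected lookup of the player character's HealthComponent is left unused.
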(event Custom|CustomEvent
  ;[0.15 0.15 0.15 0.5] Таймер игры
  (bind _output_get (Variables|Default|SetGameTime (- (Variables|Default|GetGameTime) 1)))
  (if (== _output_get 0)
    (Utilities|Time|ClearandInvalidateTimerbyHandle (Variables|Default|GetTimerHandle))
    (bind _returnvalue (UserInterface|CreateWidget "/Game/LeaveMeAlone/Widgets/UI/WBP_EndOfGame.WBP_EndOfGame_C"))
    (UserInterface|Viewport|AddtoViewport _returnvalue 0)
    (bind _aspc_leave_me_alone (Utilities|Casting|CastToPC_LeaveMeAlone (Game|GetPlayerController 0)))
    (Input|SetInputModeGameandUI _aspc_leave_me_alone _returnvalue "DoNotLock" true false)))

(event EventBeginPlay
  ;[0.15 0.15 0.15 0.5] Таймер игры
  (bind _returnvalue (Utilities|Time|SetTimerbyEvent (delegate Custom|CustomEvent) 1.0 true))
  (Variables|Default|SetTimerHandle _returnvalue))

(fn ConstructionScript)